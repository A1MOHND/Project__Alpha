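; A moving blade trap character for the Stylized Egypt level that wanders around on its own.
; On BeginPlay, two RotatingMovement components are assigned to spin separate blade meshes.
; A one-second looping timer issues an AI move to a random reachable point within a radius of the trap's current location.
; A Moving flag is set when each move starts and cleared on success or failure, though nothing in this graph reads it.
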(event Custom|Loop
  (Variables|Default|SetMoving? true)
  (AI|AIMoveTo self (.RandomLocation (AI|Navigation|GetRandomReachablePointinRadius (Transformation|GetActorLocation) 2e+03 0 0)) 0 5.0 false
    (:OnSuccess
      _)
    (:OnFail
      _))
  (Variables|Default|SetMoving? false))

(event EventBeginPlay
  (Utilities|FlowControl|Sequence
    (:then_0
      (Components|Movement|SetUpdatedComponent (Variables|Default|GetRotatingMovement) (Variables|Default|GetSM_Blade_02))
      (Components|Movement|SetUpdatedComponent (Variables|Default|GetRotatingMovement1) (Variables|Default|GetSM_Blade_03)))
    (:then_1
      (Utilities|Time|SetTimerbyEvent (delegate Custom|Loop) 1.0 true))))

(fn ConstructionScript)