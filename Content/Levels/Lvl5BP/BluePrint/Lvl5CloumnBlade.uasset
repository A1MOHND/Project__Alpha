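; Level 5 column blade hazard that spins four meshes and damages the player character on contact.
; Construction script sets an InterpToMovement path between two relative location variables, and BeginPlay binds a RotatingMovement component to each mesh.
; Three box overlaps each deal random damage to a non-ragdolled TheCharecter, gated by their own DoOnce that resets after a delay.
; Only the first box also sets the Fix flag.
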(event OnComponentBeginOverlap(Box)
  (params (OverlappedComponent :type Primitive%20Component%20Object%20Reference) (OtherActor :type Actor%20Object%20Reference) (OtherComp :type Primitive%20Component%20Object%20Reference) (OtherBodyIndex :type Integer) (bFromSweep :type Boolean) (SweepResult :type Hit%20Result%20Structure%20%28by%20ref%29))
  (bind _asthe_charecter (Utilities|Casting|CastToTheCharecter OtherActor))
  (if (not (Variables|/Game/TheCharecter/Blueprints/TheCharecter.TheCharecter_C|GetRagdoll _asthe_charecter))
    (Utilities|FlowControl|DoOnce false :!label _label
      (:Completed
        (Game|Damage|ApplyDamage _asthe_charecter (Math|Random|RandomFloatinRange 3e+01 6e+01) 0 0)
        (Variables|Default|SetFix true)
        (Utilities|FlowControl|Delay 3.0)
        (goto _label Reset)))))

(event OnComponentBeginOverlap(Box2)
  (params (OverlappedComponent :type Primitive%20Component%20Object%20Reference) (OtherActor :type Actor%20Object%20Reference) (OtherComp :type Primitive%20Component%20Object%20Reference) (OtherBodyIndex :type Integer) (bFromSweep :type Boolean) (SweepResult :type Hit%20Result%20Structure%20%28by%20ref%29))
  (bind _asthe_charecter (Utilities|Casting|CastToTheCharecter OtherActor))
  (if (not (Variables|/Game/TheCharecter/Blueprints/TheCharecter.TheCharecter_C|GetRagdoll _asthe_charecter))
    (Utilities|FlowControl|DoOnce false :!label _label
      (:Completed
        (Game|Damage|ApplyDamage _asthe_charecter (Math|Random|RandomFloatinRange 3e+01 6e+01) 0 0)
        (Utilities|FlowControl|Delay 3.0)
        (goto _label Reset)))))

(event OnComponentBeginOverlap(Box1)
  (params (OverlappedComponent :type Primitive%20Component%20Object%20Reference) (OtherActor :type Actor%20Object%20Reference) (OtherComp :type Primitive%20Component%20Object%20Reference) (OtherBodyIndex :type Integer) (bFromSweep :type Boolean) (SweepResult :type Hit%20Result%20Structure%20%28by%20ref%29))
  (bind _asthe_charecter (Utilities|Casting|CastToTheCharecter OtherActor))
  (if (not (Variables|/Game/TheCharecter/Blueprints/TheCharecter.TheCharecter_C|GetRagdoll _asthe_charecter))
    (Utilities|FlowControl|DoOnce false :!label _label
      (:Completed
        (Game|Damage|ApplyDamage _asthe_charecter (Math|Random|RandomFloatinRange 3e+01 6e+01) 0 0)
        (Utilities|FlowControl|Delay 3.0)
        (goto _label Reset)))))

(event EventBeginPlay
  (Components|Movement|SetUpdatedComponent (Variables|Default|GetRotatingMovement) (Variables|Default|GetStaticMesh1))
  (Components|Movement|SetUpdatedComponent (Variables|Default|GetRotatingMovement1) (Variables|Default|GetStaticMesh2))
  (Components|Movement|SetUpdatedComponent (Variables|Default|GetRotatingMovement2) (Variables|Default|GetStaticMesh))
  (Components|Movement|SetUpdatedComponent (Variables|Default|GetRotatingMovement3) (Variables|Default|GetStaticMesh3)))

(fn ConstructionScript
  (bind _interptomovement (Variables|Default|GetInterpToMovement))
  (Variables|/Script/Engine.InterpToMovementComponent|SetControlPoints _interptomovement (Utilities|Array|MakeArray (Utilities|Struct|MakeInterpControlPoint (Variables|Default|GetLocatoin1) true) (Utilities|Struct|MakeInterpControlPoint (Variables|Default|GetLocatoin2) true)))
  (Variables|/Script/Engine.InterpToMovementComponent|SetDuration _interptomovement 3.0))