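; Swinging ball-and-chain trap that damages TheCharecter on contact.
; A timeline started on BeginPlay drives the chain mesh's pitch through a half-turn arc, and a LoopMovement event restarts it from the beginning.
; A box overlap applies damage unless the character is ragdolled, with a DoOnce and short delay acting as a cooldown between hits.
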(event OnComponentBeginOverlap(Box)
  (params (OverlappedComponent :type Primitive%20Component%20Object%20Reference) (OtherActor :type Actor%20Object%20Reference) (OtherComp :type Primitive%20Component%20Object%20Reference) (OtherBodyIndex :type Integer) (bFromSweep :type Boolean) (SweepResult :type Hit%20Result%20Structure%20%28by%20ref%29))
  (bind _asthe_charecter (Utilities|Casting|CastToTheCharecter OtherActor))
  (if (not (Variables|/Game/TheCharecter/Blueprints/TheCharecter.TheCharecter_C|GetRagdoll _asthe_charecter))
    (Utilities|FlowControl|DoOnce false :!label _label
      (:Completed
        (Game|Damage|ApplyDamage _asthe_charecter 1e+01 0 0)
        (Utilities|FlowControl|Delay 1.0)
        (goto _label Reset)))))

(event Custom|LoopMovement
  (bind _float (Timeline|Timeline_0 PlayFromStart)
    (:Update
      (Transformation|SetRelativeRotation (Variables|Default|GetLinks_And_Modular_Chain_LOD0_uc1uegjhx_13) (Math|Rotator|MakeRotator 0.0 (Math|Float|Lerp 0.0 -1.8e+02 _float) 1.8e+02) false false))))

(event EventBeginPlay
  (bind _float (Timeline|Timeline_0 PlayFromStart)
    (:Update
      (Transformation|SetRelativeRotation (Variables|Default|GetLinks_And_Modular_Chain_LOD0_uc1uegjhx_13) (Math|Rotator|MakeRotator 0.0 (Math|Float|Lerp 0.0 -1.8e+02 _float) 1.8e+02) false false))))

(fn ConstructionScript)