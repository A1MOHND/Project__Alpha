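; WaterBP is a level water hazard that removes the player character when TheCharecter enters its Box trigger.
; The overlap checks that the character is not Dead, then passes a DoOnce gate so it fires once.
; It disables input on player 0's character, rather than using the overlapping reference, waits briefly, destroys that character and sets flag A.
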(event OnComponentBeginOverlap(Box)
  (params (OverlappedComponent :type Primitive%20Component%20Object%20Reference) (OtherActor :type Actor%20Object%20Reference) (OtherComp :type Primitive%20Component%20Object%20Reference) (OtherBodyIndex :type Integer) (bFromSweep :type Boolean) (SweepResult :type Hit%20Result%20Structure%20%28by%20ref%29))
  (bind _asthe_charecter (Utilities|Casting|CastToTheCharecter OtherActor))
  (if (not (Variables|/Game/TheCharecter/Blueprints/TheCharecter.TheCharecter_C|GetDead _asthe_charecter))
    (Utilities|FlowControl|DoOnce false
      (:Completed
        (Input|DisableInput (Game|GetPlayerCharacter 0) (Game|GetPlayerController 0))
        (Utilities|FlowControl|Delay 0.13)
        (Actor|DestroyActor (Game|GetPlayerCharacter 0))
        (Variables|Default|SetA true)))))

(fn ConstructionScript)