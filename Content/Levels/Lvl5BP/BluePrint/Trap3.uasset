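; Level 5 trap with two spinning blades that travels along a spline and damages the player character.
; RotatingMovement components spin the blades, while a timeline with play rate 1/Time drives the actor's position and rotation along the Spline actor found by GetActorOfClass at BeginPlay.
; Two box overlaps deal random damage to non-ragdolled characters, each behind a DoOnce that resets one second after a hit but stays closed if a ragdolled character triggers it.
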(event OnComponentBeginOverlap(Box)
  (params (OverlappedComponent :type Primitive%20Component%20Object%20Reference) (OtherActor :type Actor%20Object%20Reference) (OtherComp :type Primitive%20Component%20Object%20Reference) (OtherBodyIndex :type Integer) (bFromSweep :type Boolean) (SweepResult :type Hit%20Result%20Structure%20%28by%20ref%29))
  (bind _asthe_charecter (Utilities|Casting|CastToTheCharecter OtherActor))
  (Utilities|FlowControl|DoOnce false :!label _label
    (:Completed
      (if (not (Variables|/Game/TheCharecter/Blueprints/TheCharecter.TheCharecter_C|GetRagdoll _asthe_charecter))
        (Game|Damage|ApplyDamage _asthe_charecter (Math|Random|RandomFloatinRange 25.0 37.0) 0 0)
        (Utilities|FlowControl|Delay 1.0)
        (goto _label Reset)))))

(event OnComponentBeginOverlap(Box1)
  (params (OverlappedComponent :type Primitive%20Component%20Object%20Reference) (OtherActor :type Actor%20Object%20Reference) (OtherComp :type Primitive%20Component%20Object%20Reference) (OtherBodyIndex :type Integer) (bFromSweep :type Boolean) (SweepResult :type Hit%20Result%20Structure%20%28by%20ref%29))
  (bind _asthe_charecter (Utilities|Casting|CastToTheCharecter OtherActor))
  (Utilities|FlowControl|DoOnce false :!label _label
    (:Completed
      (if (not (Variables|/Game/TheCharecter/Blueprints/TheCharecter.TheCharecter_C|GetRagdoll _asthe_charecter))
        (Game|Damage|ApplyDamage _asthe_charecter (Math|Random|RandomFloatinRange 25.0 37.0) 0 0)
        (Utilities|FlowControl|Delay 1.0)
        (goto _label Reset)))))

(event Custom|MoveObject
  (bind _splinereff (Variables|Default|GetSplineReff))
  (bind _spline (Variables|/Game/Levels/Levl1BP/Stylized_Egypt/BluePrint/Spline.Spline_C|GetSpline _splinereff))
  (Components|Timeline|SetPlayRate (Variables|Default|GetTimeline_0) (/ 1.0 (Variables|Default|GetTime)))
  (bind _newtrack_0 (Timeline|Timeline_0 Play)
    (:Update
      (Transformation|SetActorTransform (Math|Transform|MakeTransform (Spline|GetLocationatDistanceAlongSpline _spline (Math|Float|Lerp (* _newtrack_0 -1.0) (Spline|GetSplineLength (Variables|/Game/Levels/Levl1BP/Stylized_Egypt/BluePrint/Spline.Spline_C|GetSpline (Variables|Default|GetSplineReff))) _newtrack_0) "World") (Spline|GetRotationatDistanceAlongSpline _spline (Math|Float|Lerp (* _newtrack_0 -1.0) (Spline|GetSplineLength (Variables|/Game/Levels/Levl1BP/Stylized_Egypt/BluePrint/Spline.Spline_C|GetSpline (Variables|Default|GetSplineReff))) _newtrack_0) "World") "1,1,1")))))

(event EventBeginPlay
  (Utilities|FlowControl|Sequence
    (:then_0
      (Components|Movement|SetUpdatedComponent (Variables|Default|GetRotatingMovement) (Variables|Default|GetSM_Blade_02))
      (Components|Movement|SetUpdatedComponent (Variables|Default|GetRotatingMovement1) (Variables|Default|GetSM_Blade_03)))
    (:then_1
      (bind _returnvalue (Actor|GetActorOfClass "/Game/Levels/Levl1BP/Stylized_Egypt/BluePrint/Spline.Spline_C"))
      (Variables|Default|SetSplineReff _returnvalue)
      (CallFunction|MoveObject))))

(fn ConstructionScript)