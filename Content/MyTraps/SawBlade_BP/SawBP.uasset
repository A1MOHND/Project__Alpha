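; Saw blade trap that slides between two configurable points and damages the player character on contact.
; The construction script feeds two relative location variables into an InterpToMovement component as control points with a fixed travel duration.
; Box overlap applies random damage to a non-ragdolled TheCharecter, with a DoOnce reset after a short delay acting as a hit cooldown.
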(event OnComponentBeginOverlap(Box)
  (params (OverlappedComponent :type Primitive%20Component%20Object%20Reference) (OtherActor :type Actor%20Object%20Reference) (OtherComp :type Primitive%20Component%20Object%20Reference) (OtherBodyIndex :type Integer) (bFromSweep :type Boolean) (SweepResult :type Hit%20Result%20Structure%20%28by%20ref%29))
  (bind _asthe_charecter (Utilities|Casting|CastToTheCharecter OtherActor))
  (if (not (Variables|/Game/TheCharecter/Blueprints/TheCharecter.TheCharecter_C|GetRagdoll _asthe_charecter))
    (Utilities|FlowControl|DoOnce false :!label _label
      (:Completed
        (Game|Damage|ApplyDamage _asthe_charecter (Math|Random|RandomFloatinRange 18.0 3e+01) 0 0)
        (Utilities|FlowControl|Delay 0.5)
        (goto _label Reset)))))

(event EventBeginPlay)

(fn ConstructionScript
  (bind _interptomovement (Variables|Default|GetInterpToMovement))
  (Variables|/Script/Engine.InterpToMovementComponent|SetControlPoints _interptomovement (Utilities|Array|MakeArray (Utilities|Struct|MakeInterpControlPoint (Variables|Default|GetLocatoin1) true) (Utilities|Struct|MakeInterpControlPoint (Variables|Default|GetLocatoin2) true)))
  (Variables|/Script/Engine.InterpToMovementComponent|SetDuration _interptomovement 1.0))