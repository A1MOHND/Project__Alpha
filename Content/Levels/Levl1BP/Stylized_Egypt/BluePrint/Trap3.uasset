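; Trap actor for an Egypt-themed level that moves itself along a spline path, starting at BeginPlay.
; It finds the level's Spline actor with GetActorOfClass, so it follows whichever instance that call returns.
; A timeline, with play rate set to the inverse of a Time variable, lerps distance toward the spline's length.
; Each update sets the actor's location in world space but takes rotation from the spline in local space.
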(event Custom|MoveObject
  (bind _splinereff (Variables|Default|GetSplineReff))
  (bind _spline (Variables|/Game/Levels/Levl1BP/Stylized_Egypt/BluePrint/Spline.Spline_C|GetSpline _splinereff))
  (Components|Timeline|SetPlayRate (Variables|Default|GetTimeline_0) (/ 1.0 (Variables|Default|GetTime)))
  (bind _newtrack_0 (Timeline|Timeline_0 Play)
    (:Update
      (Transformation|SetActorTransform (Math|Transform|MakeTransform (Spline|GetLocationatDistanceAlongSpline _spline (Math|Float|Lerp (* _newtrack_0 -1.0) (Spline|GetSplineLength (Variables|/Game/Levels/Levl1BP/Stylized_Egypt/BluePrint/Spline.Spline_C|GetSpline (Variables|Default|GetSplineReff))) _newtrack_0) "World") (Spline|GetRotationatDistanceAlongSpline _spline (Math|Float|Lerp (* _newtrack_0 -1.0) (Spline|GetSplineLength (Variables|/Game/Levels/Levl1BP/Stylized_Egypt/BluePrint/Spline.Spline_C|GetSpline (Variables|Default|GetSplineReff))) _newtrack_0) "Local") "1,1,1")))))

(event EventBeginPlay
  (bind _returnvalue (Actor|GetActorOfClass "/Game/Levels/Levl1BP/Stylized_Egypt/BluePrint/Spline.Spline_C"))
  (Variables|Default|SetSplineReff _returnvalue)
  (CallFunction|MoveObject))

(fn ConstructionScript)