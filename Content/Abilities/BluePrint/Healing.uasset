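; Healing pickup Blueprint that restores health to the player when a TheCharecter overlaps its Box trigger while below full health.
; It adds a fixed amount to player character 0's Health rather than the overlapping actor's, clamping it to the maximum.
; It plays a 2D healing sound, spawns a HeallingEffect actor at its own transform, then destroys itself.
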(event OnComponentBeginOverlap(Box)
  (params (OverlappedComponent :type Primitive%20Component%20Object%20Reference) (OtherActor :type Actor%20Object%20Reference) (OtherComp :type Primitive%20Component%20Object%20Reference) (OtherBodyIndex :type Integer) (bFromSweep :type Boolean) (SweepResult :type Hit%20Result%20Structure%20%28by%20ref%29))
  (bind _returnvalue (Game|GetPlayerCharacter 0))
  (bind _asthe_charecter (Utilities|Casting|CastToTheCharecter _returnvalue))
  (bind _asthe_charecter_2 (Utilities|Casting|CastToTheCharecter OtherActor))
  (if (< (Variables|/Game/TheCharecter/Blueprints/TheCharecter.TheCharecter_C|GetHealth _asthe_charecter_2) 1e+02)
    (Variables|/Game/TheCharecter/Blueprints/TheCharecter.TheCharecter_C|SetHealth _asthe_charecter (+ (Variables|/Game/TheCharecter/Blueprints/TheCharecter.TheCharecter_C|GetHealth _asthe_charecter) 5e+01))
    (Audio|PlaySound2D "/Game/Abilities/BluePrint/Sounds/Healing_15.Healing_15" 1.0 1.0 0.0 0 0)
    (Game|SpawnActorfromClass "/Game/Abilities/BluePrint/HeallingEffect.HeallingEffect_C" (Transformation|GetActorTransform) "Undefined" 0 0)
    (if (> (Variables|/Game/TheCharecter/Blueprints/TheCharecter.TheCharecter_C|GetHealth (.AsThe%20Charecter (Utilities|Casting|CastToTheCharecter (Game|GetPlayerCharacter 0)))) 1e+02)
      (Variables|/Game/TheCharecter/Blueprints/TheCharecter.TheCharecter_C|SetHealth (.AsThe%20Charecter (Utilities|Casting|CastToTheCharecter (Game|GetPlayerCharacter 0))) 1e+02)
      (Actor|DestroyActor)
      (else
        (Actor|DestroyActor)))))

(fn ConstructionScript)