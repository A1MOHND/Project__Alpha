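; Floor spike trap that raises its spikes and damages TheCharecter when the player character steps on it.
; Overlapping Box sets Active and plays a timeline lifting SMSpikes, while leaving clears Active and reverses it after a delay.
; Box1 overlap passes a DoOnce, waits, then applies random damage if still Active.
; The DoOnce resets after a cooldown only when damage was dealt.
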(event OnComponentBeginOverlap(Box)
  (params (OverlappedComponent :type Primitive%20Component%20Object%20Reference) (OtherActor :type Actor%20Object%20Reference) (OtherComp :type Primitive%20Component%20Object%20Reference) (OtherBodyIndex :type Integer) (bFromSweep :type Boolean) (SweepResult :type Hit%20Result%20Structure%20%28by%20ref%29))
  (Utilities|Casting|CastToTheCharecter OtherActor)
  (Variables|Default|SetActive true)
  (bind _newtrack_0 (Timeline|Timeline_0 Play)
    (:Update
      (Transformation|SetRelativeLocation (Variables|Default|GetSM_Spikes) (Math|Vector|MakeVector 0.0 0.0 (Math|Float|Lerp 0.0 8e+01 _newtrack_0)) false false))))

(event OnComponentBeginOverlap(Box1)
  (params (OverlappedComponent :type Primitive%20Component%20Object%20Reference) (OtherActor :type Actor%20Object%20Reference) (OtherComp :type Primitive%20Component%20Object%20Reference) (OtherBodyIndex :type Integer) (bFromSweep :type Boolean) (SweepResult :type Hit%20Result%20Structure%20%28by%20ref%29))
  (bind _asthe_charecter (Utilities|Casting|CastToTheCharecter OtherActor))
  (Utilities|FlowControl|DoOnce false :!label _label
    (:Completed
      (Utilities|FlowControl|Delay 1.0)
      (if (Variables|Default|GetActive)
        (Game|Damage|ApplyDamage _asthe_charecter (Math|Random|RandomFloatinRange 28.0 4e+01) 0 0)
        (Utilities|FlowControl|Delay 2.0)
        (goto _label Reset)))))

(event OnComponentEndOverlap(Box)
  (params (OverlappedComponent :type Primitive%20Component%20Object%20Reference) (OtherActor :type Actor%20Object%20Reference) (OtherComp :type Primitive%20Component%20Object%20Reference) (OtherBodyIndex :type Integer))
  (Utilities|Casting|CastToTheCharecter OtherActor)
  (Variables|Default|SetActive false)
  (Utilities|FlowControl|Delay 1.0)
  (bind _newtrack_0 (Timeline|Timeline_0 Reverse)
    (:Update
      (Transformation|SetRelativeLocation (Variables|Default|GetSM_Spikes) (Math|Vector|MakeVector 0.0 0.0 (Math|Float|Lerp 0.0 8e+01 _newtrack_0)) false false))))

(event EventBeginPlay)

(fn ConstructionScript)