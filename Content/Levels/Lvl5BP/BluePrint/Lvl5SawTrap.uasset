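; Saw trap for level 5 that spins while moving along a path between two points.
; The construction script gives InterpToMovement two relative control points from the location variables and a fixed travel duration.
; On BeginPlay, a timeline drives the roll of the Scene component's relative rotation through two full turns to produce the spin.
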(event EventBeginPlay
  (bind _newtrack_0 (Timeline|Timeline_0 Play)
    (:Update
      (Transformation|SetRelativeRotation (Variables|Default|GetScene) (Math|Rotator|MakeRotator (Math|Float|Lerp 3.6e+02 -3.6e+02 _newtrack_0) 0.0 0.0) false false))))

(fn ConstructionScript
  (bind _interptomovement (Variables|Default|GetInterpToMovement))
  (Variables|/Script/Engine.InterpToMovementComponent|SetControlPoints _interptomovement (Utilities|Array|MakeArray (Utilities|Struct|MakeInterpControlPoint (Variables|Default|GetLocatoin1) true) (Utilities|Struct|MakeInterpControlPoint (Variables|Default|GetLocatoin2) true)))
  (Variables|/Script/Engine.InterpToMovementComponent|SetDuration _interptomovement 1.5))