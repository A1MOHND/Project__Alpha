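; DoorBlade is a one-shot blade trap that slides two sword meshes out and back when TheCharecter enters its Box trigger.
; Timelines chained from Update pins extend both swords almost together, then retract them after delays.
; A second trigger, Box2, deals random damage to the character once, only while Active is false.
; Active turns true shortly after extension starts and is never reset here, closing the damage window.
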(event OnComponentBeginOverlap(Box)
  (params (OverlappedComponent :type Primitive%20Component%20Object%20Reference) (OtherActor :type Actor%20Object%20Reference) (OtherComp :type Primitive%20Component%20Object%20Reference) (OtherBodyIndex :type Integer) (bFromSweep :type Boolean) (SweepResult :type Hit%20Result%20Structure%20%28by%20ref%29))
  (Utilities|Casting|CastToTheCharecter OtherActor)
  (Utilities|FlowControl|DoOnce false
    (:Completed
      (bind _newtrack_0 (Timeline|Timeline_0 Play)
        (:Update
          (Transformation|SetRelativeLocation (Variables|Default|GetSM_Sword) (Math|Vector|MakeVector (Math|Float|Lerp 0.0 3.5e+02 _newtrack_0) 0.0 0.0) false false)
          (bind _newtrack_0_2 (Timeline|Timeline_1 Play)
            (:Update
              (Transformation|SetRelativeLocation (Variables|Default|GetSM_Sword1) (Math|Vector|MakeVector (Math|Float|Lerp -1e-05 3.5e+02 _newtrack_0_2) 0.0 -1.6e+02) false false)
              (Utilities|FlowControl|Delay 0.6)
              (Variables|Default|SetActive true)
              (Utilities|FlowControl|Delay 2.0)
              (bind _newtrack_0_3 (Timeline|Timeline_2 Play)
                (:Update
                  (Transformation|SetRelativeLocation (Variables|Default|GetSM_Sword) (Math|Vector|MakeVector (Math|Float|Lerp 3.5e+02 0.0 _newtrack_0_3) 0.0 0.0) false false)
                  (bind _newtrack_0_4 (Timeline|Timeline_3 Play)
                    (:Update
                      (Transformation|SetRelativeLocation (Variables|Default|GetSM_Sword1) (Math|Vector|MakeVector (Math|Float|Lerp 3.5e+02 -1e-05 _newtrack_0_4) 0.0 -1.6e+02) false false))))))))))))

(event OnComponentBeginOverlap(Box2)
  (params (OverlappedComponent :type Primitive%20Component%20Object%20Reference) (OtherActor :type Actor%20Object%20Reference) (OtherComp :type Primitive%20Component%20Object%20Reference) (OtherBodyIndex :type Integer) (bFromSweep :type Boolean) (SweepResult :type Hit%20Result%20Structure%20%28by%20ref%29))
  (bind _asthe_charecter (Utilities|Casting|CastToTheCharecter OtherActor))
  (if (not (Variables|Default|GetActive))
    (Utilities|FlowControl|DoOnce false
      (:Completed
        (Game|Damage|ApplyDamage _asthe_charecter (Math|Random|RandomFloatinRange 3e+01 5e+01) 0 0)))))

(fn ConstructionScript)