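; Game mode that runs the player's death and respawn sequence when the player character is destroyed.
; On BeginPlay it binds to the character's destroyed event, then skips the sequence if a flag on the TELE actor is set.
; Otherwise it fades the camera out, adds an audio component and briefly shows YouDieWidget.
; After that delay it hands the actual respawn to CharecterController.
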(event Custom|Respawn
  (params (DestroyedActor :type Actor%20Object%20Reference))
  (bind _returnvalue (Actor|GetActorOfClass "/Game/Teeleport/TELE.TELE_C"))
  (if (not (Variables|/Game/Teeleport/TELE.TELE_C|Get11 _returnvalue))
    (CameraFades|StartCameraFade :self (Game|GetPlayerCameraManager 0) :ToAlpha 1.0 :Duration 1.0 :bHoldWhenFinished true)
    (AddComponent|AddAudioComponent false)
    (bind _returnvalue_2 (UserInterface|CreateWidget "/Game/UI/DeathWidge/YouDieWidget.YouDieWidget_C"))
    (bind _output_get (Variables|Default|SetW1 _returnvalue_2))
    (UserInterface|Viewport|AddtoViewport _output_get 0)
    (Utilities|FlowControl|Delay 2.0)
    (Widget|RemovefromParent (Variables|Default|GetW1))
    (bind _ascharecter_controller (Utilities|Casting|CastToCharecterController (Game|GetPlayerController 0)))
    (Default|Respawn _ascharecter_controller)))

(event EventBeginPlay
  (Game|AssignOnDestroyed (Game|GetPlayerCharacter 0) (delegate Custom|Respawn)))

(fn ConstructionScript)