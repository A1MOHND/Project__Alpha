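; Protect is a pickup actor that grants TheCharecter a protection ability on overlap.
; Its Box overlap handler destroys any actor tagged "G" that touches it.
; For other actors, it casts to TheCharecter and requires Health above zero and Abilite2 not set.
; It then plays a magic sound, calls Protect on the character and destroys itself.
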(event OnComponentBeginOverlap(Box)
  (params (OverlappedComponent :type Primitive%20Component%20Object%20Reference) (OtherActor :type Actor%20Object%20Reference) (OtherComp :type Primitive%20Component%20Object%20Reference) (OtherBodyIndex :type Integer) (bFromSweep :type Boolean) (SweepResult :type Hit%20Result%20Structure%20%28by%20ref%29))
  (if (Actor|ActorHasTag OtherActor "G")
    (Actor|DestroyActor OtherActor)
    (else
      (bind _asthe_charecter (Utilities|Casting|CastToTheCharecter OtherActor))
      (if (not (or (<= (Variables|/Game/TheCharecter/Blueprints/TheCharecter.TheCharecter_C|GetHealth _asthe_charecter) 0.0) (Variables|/Game/TheCharecter/Blueprints/TheCharecter.TheCharecter_C|GetAbilite2 _asthe_charecter)))
        (Audio|PlaySound2D "/Game/Abilities/BluePrint/Sounds/Magic_Element_4_2.Magic_Element_4_2" 1.0 1.0 0.0 0 0)
        (Default|Protect _asthe_charecter)
        (Actor|DestroyActor)))))

(fn ConstructionScript)